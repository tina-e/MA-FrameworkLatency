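; Character Blueprint that fills a fixed volume with randomly colored rectangles while the left mouse button is held.
; On press it spawns a thousand BP_Rect actors at random points with random scale, each given a dynamic material instance with a random color.
; It also spawns one large, fixed-position white rectangle.
; On release it destroys every BP_Rect in the world.
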(event `self.ReceiveBeginPlay`)

(event `Key|LeftMouseButton`
  (params (Key :type "Key Structure"))
  (:`Pressed`
    (for _ (range 1000)
      (bind _returnvalue (`|SpawnActorFromClass` "/Game/rects/BP_Rect.BP_Rect_C" (`KismetMathLibrary.Conv_VectorToTransform` (`KismetMathLibrary.RandomPointInBoundingBox` (1100.0 180.0 0.0) (200.0 920.0 540.0))) "Undefined" "MultiplyWithRoot" null null))
      (`self.K2_SetActorRotation` _returnvalue (struct :`Pitch` 90.0) false)
      (`self.SetActorScale3D` _returnvalue (`KismetMathLibrary.MakeVector` (`KismetMathLibrary.RandomFloatInRange` 0.5 2.0) (`KismetMathLibrary.RandomFloatInRange` 0.5 2.0) (`KismetMathLibrary.RandomFloatInRange` 0.5 2.0)))
      (bind _returnvalue_2 (`PrimitiveComponent.CreateDynamicMaterialInstance` (`/Game/rects/BP_Rect.Plane` _returnvalue) 0 "/Game/asstes/dynamic_mat_instance.dynamic_mat_instance" "None"))
      (`MaterialInstanceDynamic.SetVectorParameterValue` _returnvalue_2 "color" (`KismetMathLibrary.MakeColor` (`KismetMathLibrary.RandomFloat`) (`KismetMathLibrary.RandomFloat`) (`KismetMathLibrary.RandomFloat`))))
    (bind _returnvalue_3 (`|SpawnActorFromClass` "/Game/rects/BP_Rect.BP_Rect_C" (`KismetMathLibrary.Conv_VectorToTransform` (`KismetMathLibrary.MakeVector` 899.0 -1100.0 480.0)) "Undefined" "MultiplyWithRoot" null null))
    (`self.SetActorScale3D` _returnvalue_3 (`KismetMathLibrary.MakeVector` 100.0 5.0 10.0))
    (`PrimitiveComponent.SetMaterial` (`/Game/rects/BP_Rect.Plane` _returnvalue_3) 0 "/Game/asstes/white_material.white_material")
    (`self.K2_SetActorRotation` _returnvalue_3 (struct :`Pitch` 90.0) false))
  (:`Released`
    (bind _outactors (`GameplayStatics.GetAllActorsOfClass` "/Game/rects/BP_Rect.BP_Rect_C"))
    (for _array_element _outactors
      (`self.K2_DestroyActor` _array_element))))

(fn `UserConstructionScript`)